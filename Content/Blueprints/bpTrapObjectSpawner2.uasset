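; Timed proximity trap that damages the player who comes near it while it is in its red, monitoring state.
; One looping timer toggles the monitoring state every few seconds and recolors the Spawner sprite red or green to show it.
; A second, fast looping timer compares squared distance to player 0 and applies heavy damage through MyCharacter when within range and monitoring.
; Despite its name it spawns nothing, and the stored start position is unused.
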(event `self.ReceiveBeginPlay`
  (`PaperSpriteComponent.SetSpriteColor` (`self.Spawner`) (struct :`R` 1.0 :`A` 1.0))
  (set `self.IsMonitoring` true)
  (set `self.StartPos` (`self.K2_GetActorLocation`))
  (`KismetSystemLibrary.K2_SetTimer` null "FireMonitor" 5.0 true)
  (`KismetSystemLibrary.K2_SetTimer` null "CheckPlayerCollision" 0.1 true))

(event `FireMonitor`
  (if (`self.IsMonitoring`)
    (`PaperSpriteComponent.SetSpriteColor` (`self.Spawner`) (struct :`G` 0.95 :`B` 0.049263 :`A` 1.0))
    (set `self.IsMonitoring` false)
    (else
      (`PaperSpriteComponent.SetSpriteColor` (`self.Spawner`) (struct :`R` 1.0 :`G` 0.020778 :`B` 0.030725 :`A` 1.0))
      (set `self.IsMonitoring` true))))

(event `CheckPlayerCollision`
  (bind _returnvalue (`GameplayStatics.GetPlayerCharacter` 0))
  (if (<= (`KismetMathLibrary.VSizeSquared` (- (`self.K2_GetActorLocation`) (`self.K2_GetActorLocation` _returnvalue))) 44200.0)
    (if (`self.IsMonitoring`)
      (bind _asmy_character (cast `/Game/Blueprints/MyCharacter` _returnvalue))
      (`/Game/Blueprints/MyCharacter.TakeDamage` _asmy_character 100.0))))

(fn `UserConstructionScript`)