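; Enemy actor that moves along X and damages a nearby player; despite its name, it spawns nothing.
; On BeginPlay, a timeline lerps it between its start position and an X offset, flipping its rotation near the far end and resetting it at the start.
; A looping timer runs FireGameOver, which uses a squared-distance check to apply heavy damage to MyCharacter within range.
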(event `self.ReceiveBeginPlay`
  (bind _startpos (`self.StartPos`))
  (bind (_startpos_x _startpos_y _startpos_z) (`KismetMathLibrary.BreakVector` (`self.StartPos`)))
  (set `self.StartPos` (`self.K2_GetActorLocation`))
  (`KismetSystemLibrary.K2_SetTimer` null "FireGameOver" 0.1 true)
  (bind (_direction _move) (`Timeline|Timeline_0` :!via `PlayFromStart`)
    (:`Update`
      (bind _returnvalue (`KismetMathLibrary.VLerp` _startpos (`KismetMathLibrary.MakeVector` (+ _startpos_x 300.0) _startpos_y _startpos_z) _move))
      (`self.K2_SetActorLocation` _returnvalue)
      (if (== (.x _returnvalue) (.x _startpos))
        (`self.K2_SetActorRelativeRotation` (struct))
        (elif (>= (`KismetMathLibrary.VSizeSquared` (- _returnvalue _startpos)) 49000.0)
          (`self.K2_SetActorRelativeRotation` (struct :`Yaw` 180.0)))))))

(event `FireGameOver`
  (bind _returnvalue (`GameplayStatics.GetPlayerCharacter` 0))
  (if (<= (`KismetMathLibrary.VSizeSquared` (- (`self.K2_GetActorLocation` _returnvalue) (`self.K2_GetActorLocation`))) 20000.0)
    (bind _asmy_character (cast `/Game/Blueprints/MyCharacter` _returnvalue))
    (`/Game/Blueprints/MyCharacter.TakeDamage` _asmy_character 100.0)))

(fn `UserConstructionScript`)