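; Level-end trigger actor that shows the LevelComplete screen when the player gets close along the X axis, despite its spawner name.
; A looping timer started on BeginPlay compares the squared X distance to the player against a fixed threshold, ignoring Y and Z.
; On a hit it adds the widget to the viewport, disables character input, shows the mouse cursor and pauses the game.
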(event `self.ReceiveBeginPlay`
  (set `self.StartPos` (`self.K2_GetActorLocation`))
  (`KismetSystemLibrary.K2_SetTimer` null "CheckPlayerCollision" 0.1 true))

(event `CheckPlayerCollision`
  (bind _returnvalue (`GameplayStatics.GetPlayerController` 0))
  (if (<= (`KismetMathLibrary.Square` (- (.x (`self.K2_GetActorLocation`)) (.x (`self.K2_GetActorLocation` (`GameplayStatics.GetPlayerCharacter` 0))))) 150000.0)
    (bind _returnvalue_2 (`|CreateWidget` "/Game/Blueprints/Menus/LevelComplete.LevelComplete_C"))
    (`UserWidget.AddToViewport` _returnvalue_2 0)
    (`self.DisableInput` (`GameplayStatics.GetPlayerCharacter` 0) _returnvalue)
    (set `PlayerController.bShowMouseCursor` true _returnvalue)
    (`GameplayStatics.SetGamePaused` true)))

(fn `UserConstructionScript`)