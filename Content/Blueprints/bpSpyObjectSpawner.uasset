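; bpSpyObjectSpawner is a moving hazard with a red-tinted sprite that damages the player on proximity; despite its name, it spawns nothing in these graphs.
; On BeginPlay, a timeline lerps it 3000 units upward from its start position without sweeping.
; A looping timer polls squared distance to player 0 every tenth of a second, dealing 100 damage to MyCharacter on each check within roughly 316 units.
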(event `self.ReceiveBeginPlay`
  (bind (_startpos_x _startpos_y _startpos_z) (`KismetMathLibrary.BreakVector` (`self.StartPos`)))
  (`PaperSpriteComponent.SetSpriteColor` (`self.Spawner`) (struct :`R` 1.0 :`A` 1.0))
  (set `self.StartPos` (`self.K2_GetActorLocation`))
  (`KismetSystemLibrary.K2_SetTimer` null "CheckPlayerCollision" 0.1 true)
  (bind (_direction _move) (`Timeline|Timeline_0` :!via `PlayFromStart`)
    (:`Update`
      (`self.K2_SetActorLocation` (`KismetMathLibrary.VLerp` (`self.StartPos`) (`KismetMathLibrary.MakeVector` _startpos_x _startpos_y (+ _startpos_z 3000.0)) _move)))))

(event `CheckPlayerCollision`
  (bind _returnvalue (`GameplayStatics.GetPlayerCharacter` 0))
  (if (<= (`KismetMathLibrary.VSizeSquared` (- (`self.K2_GetActorLocation`) (`self.K2_GetActorLocation` _returnvalue))) 100010.0)
    (bind _asmy_character (cast `/Game/Blueprints/MyCharacter` _returnvalue))
    (`/Game/Blueprints/MyCharacter.TakeDamage` _asmy_character 100.0)))

(fn `UserConstructionScript`)