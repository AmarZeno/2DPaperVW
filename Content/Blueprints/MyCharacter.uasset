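; MyCharacter is a Paper2D side-scrolling player character that moves along the X axis and jumps.
; The MoveRight axis drives movement, flips control yaw to face the travel direction, and swaps idle and run flipbooks based on velocity.
; BeginPlay turns off replication on the Sprite component.
; A disconnected branch on HasSpot for recoloring the sprite never runs, and Tick is empty.
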(event `self.ReceiveBeginPlay`
  ;[1 1 1] Replication
  (`ActorComponent.SetIsReplicated` (`self.Sprite`) false))

(event `InputAxis|MoveRight`
  (params (AxisValue :type "Float (single-precision)"))
  ;[1 1 1] Player rotation
  (`self.AddMovementInput` (1.0 0.0 0.0) AxisValue)
  (`self.UpdateAnimation`)
  (`/Engine/EditorBlueprintResources/StandardMacros.CompareFloat` AxisValue
    (:`>`
      (`Controller.SetControlRotation` (`self.GetController`) (`KismetMathLibrary.MakeRotator` 0.0)))
    (:`<`
      (`Controller.SetControlRotation` (`self.GetController`) (`KismetMathLibrary.MakeRotator` 0.0 0.0 180.0)))))

(event `InputAction|Jump`
  (params (Key :type "Key Structure" :default "AnyKey"))
  ;[1 1 1] Jump action
  (:`Pressed`
    (`self.Jump`)))

(event `UpdateAnimation`
  (bind _aspaper_flipbook (cast `PaperFlipbook` (`KismetMathLibrary.SelectObject` "/Game/FlipBooks/RunFlipbook.RunFlipbook" "/Game/FlipBooks/IdleFlipBook.IdleFlipbook" (> (`KismetMathLibrary.VSize` (`self.GetVelocity`)) 0.0))))
  (`PaperFlipbookComponent.SetFlipbook` (`self.Sprite`) _aspaper_flipbook))

(event `self.ReceiveTick`
  (params (DeltaSeconds :type "Float (single-precision)")))

(fn `UserConstructionScript`)