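; Death box actor that damages the player character when it comes within a vertical band around the actor.
; On BeginPlay it tints its Spawner sprite red, enables monitoring and starts a looping timer.
; Each tick of that timer compares squared Z distance only, ignoring horizontal position, then applies heavy damage through MyCharacter's TakeDamage.
; Despite the name it spawns nothing, and the saved start position is never read.
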(event `self.ReceiveBeginPlay`
  (`PaperSpriteComponent.SetSpriteColor` (`self.Spawner`) (struct :`R` 1.0 :`A` 1.0))
  (set `self.IsMonitoring` true)
  (set `self.StartPos` (`self.K2_GetActorLocation`))
  (`KismetSystemLibrary.K2_SetTimer` null "CheckPlayerCollision" 0.1 true))

(event `CheckPlayerCollision`
  (bind _returnvalue (`GameplayStatics.GetPlayerCharacter` 0))
  (if (<= (`KismetMathLibrary.Square` (- (.z (`self.K2_GetActorLocation`)) (.z (`self.K2_GetActorLocation` _returnvalue)))) 88910.0)
    (if (`self.IsMonitoring`)
      (bind _asmy_character (cast `/Game/Blueprints/MyCharacter` _returnvalue))
      (`/Game/Blueprints/MyCharacter.TakeDamage` _asmy_character 100.0))))

(fn `UserConstructionScript`)